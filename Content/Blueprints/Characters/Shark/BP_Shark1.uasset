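; BP_Shark1 is a shark enemy character that targets the captain and reacts to being defeated.
; When BP_Captain enters its AggroRange, it passes the captain to its AI controller as the attack target.
; On BeginPlay it runs the parent logic and binds to the Defeated event, which moves the sprite to the relative location of the DefeatedPos component.
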(event OnComponentBeginOverlap(AggroRange)
  (params (OverlappedComponent :type Primitive%20Component%20Object%20Reference) (OtherActor :type Actor%20Object%20Reference) (OtherComp :type Primitive%20Component%20Object%20Reference) (OtherBodyIndex :type Integer) (bFromSweep :type Boolean) (SweepResult :type Hit%20Result%20Structure%20%28by%20ref%29))
  (bind _asbp_captain (Utilities|Casting|CastToBP_Captain OtherActor))
  (bind _asaic_enemy (Utilities|Casting|CastTo (AI|GetAIController self)))
  (CallFunction|SetAttackTarget _asaic_enemy _asbp_captain))

(event Custom|OnDefeated
  (Transformation|SetRelativeLocation (Variables|Default|GetSprite) (Variables|/Script/Engine.SceneComponent|GetRelativeLocation (Variables|Default|GetDefeatedPos)) false false))

(event EventBeginPlay
  (|CallParentFunction)
  (EventDispatchers|BindEventtoDefeated (delegate Custom|OnDefeated)))

(event Collision|EventActorBeginOverlap
  (params (OtherActor :type Actor%20Object%20Reference)))

(event EventTick
  (params (DeltaSeconds :type Float%20%28single-precision%29)))

(fn ConstructionScript
  (|CallParentFunction))